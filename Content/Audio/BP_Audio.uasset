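; BP_Audio is an annotated reference Blueprint that demonstrates the common nodes for controlling audio components.
; Unconnected, commented examples on MusicSpeaker cover toggling spatialization, setting a sound, play and stop, fading and volume adjustment.
; UISpeaker, AmbientSpeaker and an IsPlaying check sit unused in the graph.
; No event drives any node and the construction script is empty, so none of this logic runs.
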(fn `UserConstructionScript`)