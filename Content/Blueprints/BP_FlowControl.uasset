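; BP_FlowControl is a commented reference Blueprint demonstrating Unreal's flow-control nodes; none of its chains connect to an event, so nothing runs.
; Isolated examples cover Sequence, gates, branches, switches on string, int and enum, and loops, alongside loose boolean operators.
; A random-integer switch shows mixed case actions such as spawning, printing and quitting.
; Delay-driven feedback wires show polling and slow counting, since Delay fails inside loop bodies.
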(fn `UserConstructionScript`)