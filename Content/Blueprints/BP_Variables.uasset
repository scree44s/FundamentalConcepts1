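; BP_Variables is a reference Blueprint that lays out the common nodes for array and map variables, with none wired to an event.
; Loose node groups show array and map operations on Array1Names and Map1Inventory.
; Inventory examples treat the map as item counts: increment or insert via Find, remove only when found, and contrast removing a key with setting it to zero.
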(fn `UserConstructionScript`)